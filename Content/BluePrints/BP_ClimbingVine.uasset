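; BP_ClimbingVine is a vine actor that the main character can climb and grab.
; Box overlap flags the character as on the vine, sets Flying movement and switches input from Y to X axis.
; Leaving the box, or entering while jumping, runs shared reset logic for Walking, though that logic targets the end-overlap cast result.
; Sphere overlap toggles CanGrabVine and, on entry, registers this actor as VineGrabPoint.
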(event `self.Box.OnComponentBeginOverlap`
  (params (OverlappedComponent :type "PrimitiveComponent Object Reference") (OtherActor :type "Actor Object Reference") (OtherComp :type "PrimitiveComponent Object Reference") (OtherBodyIndex :type Integer) (bFromSweep :type Boolean) (SweepResult :type "HitResult Structure (by ref)"))
  ;[1 1 1] Allows Climbing whne the player is close enough to the object. NM
  (bind _asbp_main_character (cast `/Game/BluePrints/BP_MainCharacter` OtherActor))
  (set `/Game/BluePrints/BP_MainCharacter.OnVine` true _asbp_main_character)
  ;;[1 1 1] If the player is jumping end the overlap event
  (if (`/Game/BluePrints/BP_BaseCharacter.IsJumping` _asbp_main_character)
    (set `/Game/BluePrints/BP_MainCharacter.OnVine` false (stale `self.Box.OnComponentEndOverlap` _asbp_main_character) :!label _label)
    (`CharacterMovementComponent.SetMovementMode` (`Character.CharacterMovement` (stale `self.Box.OnComponentEndOverlap` _asbp_main_character)) "MOVE_Walking" 0)
    (set `/Game/BluePrints/BP_MainCharacter.UseYAxis` true (stale `self.Box.OnComponentEndOverlap` _asbp_main_character))
    (set `/Game/BluePrints/BP_MainCharacter.UseXAxis` false (stale `self.Box.OnComponentEndOverlap` _asbp_main_character))
    (else
      (`CharacterMovementComponent.SetMovementMode` (`Character.CharacterMovement` _asbp_main_character) "MOVE_Flying" 0)
      (set `/Game/BluePrints/BP_MainCharacter.UseYAxis` false _asbp_main_character)
      (set `/Game/BluePrints/BP_MainCharacter.UseXAxis` true _asbp_main_character))))

(event `self.Box.OnComponentEndOverlap`
  (params (OverlappedComponent :type "PrimitiveComponent Object Reference") (OtherActor :type "Actor Object Reference") (OtherComp :type "PrimitiveComponent Object Reference") (OtherBodyIndex :type Integer))
  ;[1 1 1] Allows Climbing whne the player is close enough to the object. NM
  (bind _asbp_main_character (cast `/Game/BluePrints/BP_MainCharacter` OtherActor))
  (goto _label))

(event `self.Sphere.OnComponentBeginOverlap`
  (params (OverlappedComponent :type "PrimitiveComponent Object Reference") (OtherActor :type "Actor Object Reference") (OtherComp :type "PrimitiveComponent Object Reference") (OtherBodyIndex :type Integer) (bFromSweep :type Boolean) (SweepResult :type "HitResult Structure (by ref)"))
  ;[1 1 1] Will allow the player to swing to the vine whne in range. NM
  (bind _asbp_main_character (cast `/Game/BluePrints/BP_MainCharacter` OtherActor))
  (set `/Game/BluePrints/BP_MainCharacter.CanGrabVine` true _asbp_main_character)
  (set `/Game/BluePrints/BP_MainCharacter.VineGrabPoint` self _asbp_main_character))

(event `self.Sphere.OnComponentEndOverlap`
  (params (OverlappedComponent :type "PrimitiveComponent Object Reference") (OtherActor :type "Actor Object Reference") (OtherComp :type "PrimitiveComponent Object Reference") (OtherBodyIndex :type Integer))
  ;[1 1 1] Will allow the player to swing to the vine whne in range. NM
  (bind _asbp_main_character (cast `/Game/BluePrints/BP_MainCharacter` OtherActor))
  (set `/Game/BluePrints/BP_MainCharacter.CanGrabVine` false _asbp_main_character))

(fn `UserConstructionScript`)
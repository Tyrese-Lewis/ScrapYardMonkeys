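; Player controller for a side-scroller that handles the start menu, death sequence, brightness and saved audio settings.
; BeginPlay applies the base sound mix, then restores music and effects volumes from the options save.
; StartGameSpawn opens the start menu in UI-only input with a brief fade widget, and AdjustBrightness sets gamma through a console command.
; OnDeath unpossesses, fades out and prints a message, but its restart call is unconnected.
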(event `OnDeath`
  (`self.UnPossess`)
  (`PlayerCameraManager.StartCameraFade` :`self` (`self.PlayerCameraManager`) :`ToAlpha` 1.0 :`Duration` 1.0 :`bHoldWhenFinished` true)
  (`KismetSystemLibrary.PrintString` "You Died")
  (`KismetSystemLibrary.Delay` 2.0)
  (cast `/Game/SideScrollerBP/Blueprints/SideScrollerGameMode` (`GameplayStatics.GetGameMode`)))

(event `Start Game Spawn`
  (bind _returnvalue (`GameplayStatics.GetPlayerController` 0))
  (`self.EnableInput` (`GameplayStatics.GetPlayerController` 0))
  ;[1 1 1] Create Start Menu and set game focus
  (bind _returnvalue_2 (`|CreateWidget` "/Game/Userinterface/Start_Game/Start_Menu.Start_Menu_C"))
  (`UserWidget.AddToViewport` _returnvalue_2 0)
  (set `PlayerController.bShowMouseCursor` true _returnvalue)
  (`WidgetBlueprintLibrary.SetInputMode_UIOnlyEx` _returnvalue _returnvalue_2)
  ;[1 1 1] enter effect
  (bind _returnvalue_3 (`|CreateWidget` "/Game/Userinterface/Loading/Faded_Background.Faded_Background_C"))
  (`UserWidget.AddToViewport` _returnvalue_3 0)
  (`KismetSystemLibrary.Delay` 1.0)
  (`Widget.RemoveFromParent` _returnvalue_3))

(event `Adjust Brightness`
  (params (`Control Brightness` :type "Float (double-precision)"))
  ;[1 1 1] Brightness Control
  (`KismetSystemLibrary.ExecuteConsoleCommand` (`KismetStringLibrary.Concat_StrStr` "Gamma " (`KismetStringLibrary.Conv_DoubleToString` (`KismetMathLibrary.Lerp` 0.5 5.0 `Control Brightness`))) null))

(event `self.ReceiveBeginPlay`
  ;[1 1 1] Load Audio Save Data
  (`GameplayStatics.SetBaseSoundMix` "/Game/Userinterface/Sound_Effects/SoundsMixer.SoundsMixer")
  (bind _returnvalue (`GameplayStatics.DoesSaveGameExist` (`self.SaveOptions`)))
  (if _returnvalue
    (bind _returnvalue_2 (`GameplayStatics.LoadGameFromSlot` (`self.SaveOptions`)))
    (bind _assave_game_options (cast `/Game/Userinterface/Options_Menu/SaveGameOptions` _returnvalue_2))
    (bind _output_get (set `self.Save the Options` _assave_game_options))
    (for (_array_element _array_index) (`/Game/Userinterface/Options_Menu/SaveGameOptions.Save Volume` _output_get)
      (switch `int` _array_index
        (:`0`
          (`GameplayStatics.SetSoundMixClassOverride` "/Game/Userinterface/Sound_Effects/SoundsMixer.SoundsMixer" "/Game/Userinterface/Sound_Effects/Music_Controller.Music_Controller" _array_element 1.0 0.0))
        (:`1`
          (`GameplayStatics.SetSoundMixClassOverride` "/Game/Userinterface/Sound_Effects/SoundsMixer.SoundsMixer" "/Game/Userinterface/Sound_Effects/SoundEffects_Controller.SoundEffects_Controller" _array_element 1.0 0.0))))))

(fn `UserConstructionScript`)
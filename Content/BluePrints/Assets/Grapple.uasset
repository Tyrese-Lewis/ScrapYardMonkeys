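; Grapple actor that pulls the player's side-scrolling character toward a hit point.
; On hit, it casts the player to SideScrollingCharacter_Base, sets the grapple start and end locations, and calls MoveGrapple on it.
; It then polls with a tiny looping Delay until the character's movement mode is no longer None, and destroys itself.
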(event `self.ReceiveHit`
  (params (MyComp :type "PrimitiveComponent Object Reference") (Other :type "Actor Object Reference") (OtherComp :type "PrimitiveComponent Object Reference") (bSelfMoved :type Boolean) (HitLocation :type "Vector Structure") (HitNormal :type "Vector Structure") (NormalImpulse :type "Vector Structure") (Hit :type "HitResult Structure (by ref)"))
  (bind _asside_scrolling_character_base (cast `/Game/BluePrints/Character/SideScrollingCharacter_Base` (`GameplayStatics.GetPlayerCharacter` 0)))
  (set `/Game/BluePrints/Character/SideScrollingCharacter_Base.GrappleStartLoc` (`self.K2_GetActorLocation` _asside_scrolling_character_base) _asside_scrolling_character_base)
  (set `/Game/BluePrints/Character/SideScrollingCharacter_Base.GrappleEndLoc` HitLocation _asside_scrolling_character_base)
  (`/Game/BluePrints/Character/SideScrollingCharacter_Base.MoveGrapple` _asside_scrolling_character_base)
  (`KismetSystemLibrary.Delay` 0.0001 :!label _label)
  (if (`|EnumInequality` (`CharacterMovementComponent.MovementMode` (`Character.CharacterMovement` _asside_scrolling_character_base)) "MOVE_None")
    (`self.K2_DestroyActor`)
    (else
      (goto _label))))

(fn `UserConstructionScript`)
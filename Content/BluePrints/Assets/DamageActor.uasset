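; DamageActor is a Blueprint actor that both deals and takes damage, with debug printouts of the results.
; Any actor that begins overlapping it receives a large fixed amount of damage through Apply Damage.
; Damage it receives via AnyDamage reduces its own health variable, then prints the new value and either a dead or hit message.
; Reaching zero health triggers only that printout, with no destroy logic.
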(event `self.ReceiveBeginPlay`)

(event `self.ReceiveActorBeginOverlap`
  (params (OtherActor :type "Actor Object Reference"))
  (`GameplayStatics.ApplyDamage` OtherActor 1000.0))

(event `self.ReceiveAnyDamage`
  (params (Damage :type "Float (single-precision)") (DamageType :type "DamageType Object Reference") (InstigatedBy :type "Controller Object Reference") (DamageCauser :type "Actor Object Reference"))
  (bind _output_get (set `self.CurretnHealth` (- (`self.CurretnHealth`) Damage)))
  ;[1 1 1] Debug
  (`KismetSystemLibrary.PrintString` (`KismetStringLibrary.Conv_DoubleToString` (`self.CurretnHealth`)))
  (if (<= _output_get 0.0)
    (`KismetSystemLibrary.PrintString` "Dead")
    (else
      (`KismetSystemLibrary.PrintString` "BoxTaken Damage"))))

(fn `UserConstructionScript`)
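; Bombs is a thrown explosive actor that launches along the player character's aim and detonates after a short fuse.
; On BeginPlay it sets the Bomb physics velocity from the forward vector of the side-scrolling character's Arrowend component.
; After a three-second delay it sends a damage message to actors overlapping the Boom component, spawns an emitter at the bomb's location and destroys itself.
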(event `self.ReceiveBeginPlay`
  ;[1 1 1] Bombs
  (bind _asside_scrolling_character_base (cast `/Game/BluePrints/SideScrollingCharacter_Base` (`GameplayStatics.GetPlayerCharacter` 0)))
  (`PrimitiveComponent.SetPhysicsLinearVelocity` (`self.Bomb`) (* (`SceneComponent.GetForwardVector` (`/Game/BluePrints/SideScrollingCharacter_Base.arrowend` _asside_scrolling_character_base)) 1000.0) false "None")
  (`KismetSystemLibrary.Delay` 3.0)
  (message `/Game/BluePrints/BPI_TakeDamage.TakeDamage` (`PrimitiveComponent.GetOverlappingActors` (`self.boom`) null) 20.0)
  (`GameplayStatics.SpawnEmitterAtLocation` null (`SceneComponent.K2_GetComponentLocation` (`self.Bomb`)))
  (`self.K2_DestroyActor`))

(fn `UserConstructionScript`)
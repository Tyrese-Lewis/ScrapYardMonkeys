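; Grabbable rope actor for a side-scrolling game that the player character latches onto by touching its capsule.
; On capsule overlap, if no player is connected, it checks the other actor through an IsPlayer message, sends it GrabRope with itself and marks itself connected.
; Tick overwrites that flag every frame with the Grabbing state of player 0's SideScrollingCharacter_Base.
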(event `self.ReceiveTick`
  (params (DeltaSeconds :type "Float (single-precision)"))
  (bind _asside_scrolling_character_base (cast `/Game/BluePrints/SideScrollingCharacter_Base` (`GameplayStatics.GetPlayerCharacter` 0)))
  (set `self.PlayerConnected` (`/Game/BluePrints/SideScrollingCharacter_Base.Grabbing` _asside_scrolling_character_base)))

(event `self.Capsule.OnComponentBeginOverlap`
  (params (OverlappedComponent :type "PrimitiveComponent Object Reference") (OtherActor :type "Actor Object Reference") (OtherComp :type "PrimitiveComponent Object Reference") (OtherBodyIndex :type Integer) (bFromSweep :type Boolean) (SweepResult :type "HitResult Structure (by ref)"))
  (if (not (`self.PlayerConnected`))
    (bind _true (message `/Game/BluePrints/IsPlayer.IsPlayer` OtherActor))
    (if _true
      (message `/Game/BluePrints/IsPlayer.Grab_Rope` OtherActor self)
      (set `self.PlayerConnected` true))))

(fn `UserConstructionScript`)
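; Player controller for a side-scroller that handles player death and screen brightness.
; On death it unpossesses the pawn, fades the camera to full and holds it, prints a death message, then waits briefly.
; The game mode cast after the delay leads nowhere, as the RestartGame call intended for checkpoint or level-start respawn is disconnected.
; AdjustBrightness maps the Brightness value through a Lerp into a Gamma console command.
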(event `OnDeath`
  (`self.UnPossess`)
  (`PlayerCameraManager.StartCameraFade` :`self` (`self.PlayerCameraManager`) :`ToAlpha` 1.0 :`Duration` 1.0 :`bHoldWhenFinished` true)
  (`KismetSystemLibrary.PrintString` "You Died")
  (`KismetSystemLibrary.Delay` 2.0)
  (cast `/Game/SideScrollerBP/Blueprints/SideScrollerGameMode` (`GameplayStatics.GetGameMode`)))

(event `Adjust Brightness`
  (`KismetSystemLibrary.ExecuteConsoleCommand` (`KismetStringLibrary.Concat_StrStr` "Gamma " (`KismetStringLibrary.Conv_DoubleToString` (`KismetMathLibrary.Lerp` 0.5 5.0 (`self.Brightness`)))) null))

(fn `UserConstructionScript`)
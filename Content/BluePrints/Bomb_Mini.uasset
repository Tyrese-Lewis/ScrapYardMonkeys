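; Mini bomb actor that explodes on a timer shortly after spawning.
; On BeginPlay it launches its Bomb component with a random velocity in Y and Z only, then waits through a fixed fuse delay.
; It then sends a fixed TakeDamage message to actors overlapping its Boom component, spawns an emitter at the bomb's location and destroys itself.
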(event `self.ReceiveBeginPlay`
  (bind (_returnvalue_x _returnvalue_y _returnvalue_z) (`KismetMathLibrary.BreakVector` (* (`KismetMathLibrary.RandomUnitVector`) 100.0)))
  ;[1 1 1] Bombs
  (`PrimitiveComponent.SetPhysicsLinearVelocity` (`self.Bomb`) (`KismetMathLibrary.MakeVector` 0.0 _returnvalue_y _returnvalue_z) false "None")
  (`KismetSystemLibrary.Delay` 3.0)
  (message `/Game/BluePrints/BPI_TakeDamage.TakeDamage` (`PrimitiveComponent.GetOverlappingActors` (`self.boom`) null) 10.0)
  (`GameplayStatics.SpawnEmitterAtLocation` null (`SceneComponent.K2_GetComponentLocation` (`self.Bomb`)))
  (`self.K2_DestroyActor`))

(fn `UserConstructionScript`)
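; Base character Blueprint that tracks health and handles damage and death.
; Health starts at MaxHealth on BeginPlay, and each AnyDamage event subtracts from it and prints the result for debugging.
; At zero or below, it turns off mesh physics simulation and calls OnDeath on BP_PlayerController, reached by casting the controller.
; Death and hit animations are still placeholders, marked by comments and debug prints.
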(event `self.ReceiveBeginPlay`
  (set `self.Health` (`self.MaxHealth`)))

(event `/Game/BluePrints/BPI_TakeDamage.TakeDamage`
  (params (Damage :type "Float (single-precision)"))
  ;[1 1 1] Take Damage And Apply To Health. Will Also Deal With the Death Of The Player
)

(event `self.ReceiveAnyDamage`
  (params (Damage :type "Float (single-precision)") (DamageType :type "DamageType Object Reference") (InstigatedBy :type "Controller Object Reference") (DamageCauser :type "Actor Object Reference"))
  ;[1 1 1] Take Damage And Apply To Health. Will Also Deal With the Death Of The Player
  (bind _output_get (set `self.Health` (- (`self.Health`) Damage)))
  ;;[1 1 1] Debug
  (`KismetSystemLibrary.PrintString` (`KismetStringLibrary.Conv_DoubleToString` (`self.Health`)))
  (`|ExecutionSequence`
    (:`then_1`
      (if (<= _output_get 0.0)
        ;;[1 1 1] This Will Be Replaced With the Death Animation
        (`PrimitiveComponent.SetSimulatePhysics` (`self.Mesh`) false)
        (bind _asbp_player_controller (cast `/Game/BluePrints/BP_Character/BP_PlayerController` (`self.GetController`)))
        (`/Game/BluePrints/BP_Character/BP_PlayerController.OnDeath` _asbp_player_controller)
        (`KismetSystemLibrary.PrintString` "Dead")
        (else
          ;;[1 1 1] Need To Add Damage Taken Animation Here
          (`KismetSystemLibrary.PrintString` "Taken Damage"))))))

(fn `UserConstructionScript`)
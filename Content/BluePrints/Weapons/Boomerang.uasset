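; Boomerang projectile weapon that flies out along the side-scrolling character's aim arrow and turns back toward the player.
; Its physics sphere launches on BeginPlay, is redirected once at the player's position after a short delay, and self-destroys after a timeout.
; On hit it sends damage through an interface message, then either refills boomerang ammo if the player was hit or spawns a BoomerangDropped, destroying itself.
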(event `self.ReceiveBeginPlay`
  (bind _returnvalue (`GameplayStatics.GetPlayerCharacter` 0))
  (bind _asside_scrolling_character_base (cast `/Game/BluePrints/SideScrollingCharacter_Base` _returnvalue))
  (`PrimitiveComponent.SetPhysicsLinearVelocity` (`self.Sphere`) (* (`SceneComponent.GetForwardVector` (`/Game/BluePrints/SideScrollingCharacter_Base.arrowend` _asside_scrolling_character_base)) 1000.0) false "None")
  (`KismetSystemLibrary.Delay` 0.5)
  (`PrimitiveComponent.SetPhysicsLinearVelocity` (`self.Sphere`) (* (`KismetMathLibrary.GetDirectionUnitVector` (`SceneComponent.K2_GetComponentLocation` (`self.Sphere`)) (`SceneComponent.K2_GetComponentLocation` (`Character.CapsuleComponent` _returnvalue))) 1000.0) false "None")
  (`KismetSystemLibrary.Delay` 3.0)
  (`self.K2_DestroyActor`))

(event `self.Sphere.OnComponentHit`
  (params (HitComponent :type "PrimitiveComponent Object Reference") (OtherActor :type "Actor Object Reference") (OtherComp :type "PrimitiveComponent Object Reference") (NormalImpulse :type "Vector Structure") (Hit :type "HitResult Structure (by ref)"))
  (`|ExecutionSequence`
    (:`then_0`
      (message `/Game/BluePrints/Interfaces/BPI_TakeDamage.TakeDamage` OtherActor 10.0))
    (:`then_1`
      (bind _true (message `/Game/BluePrints/Interfaces/IsPlayer.IsPlayer` OtherActor))
      (if _true
        (bind _asside_scrolling_character_base (cast `/Game/BluePrints/SideScrollingCharacter_Base` (`GameplayStatics.GetPlayerCharacter` 0)))
        (set `/Game/BluePrints/SideScrollingCharacter_Base.BoomerangAmmo` 1.0 _asside_scrolling_character_base)
        (`self.K2_DestroyActor`)
        (else
          (`|SpawnActorFromClass` "/Game/BluePrints/Weapons/BoomerangDropped.BoomerangDropped_C" (`KismetMathLibrary.MakeTransform` (`SceneComponent.K2_GetComponentLocation` (`self.Sphere`))) "Undefined" "OverrideRootScale" null null)
          (`self.K2_DestroyActor`))))))

(fn `IsPlayer`
  (returns (True :type Boolean))
  (return false))

(fn `UserConstructionScript`)
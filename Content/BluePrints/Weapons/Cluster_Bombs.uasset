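; Cluster bomb weapon actor that splits into several Bomb_Mini bomblets.
; On BeginPlay it launches its physics body along the forward vector of the side-scrolling player character's Arrowend component.
; After a three-second fuse it plays an explosion effect, scatters bomblets at random unit offsets around itself and destroys itself.
; A Sphere component hit triggers the same split immediately, but without the explosion effect.
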(event `self.ReceiveBeginPlay`
  ;[1 1 1] Bombs
  (bind _asside_scrolling_character_base (cast `/Game/BluePrints/Character/SideScrollingCharacter_Base` (`GameplayStatics.GetPlayerCharacter` 0)))
  (`PrimitiveComponent.SetPhysicsLinearVelocity` (`self.Bomb`) (* (`SceneComponent.GetForwardVector` (`/Game/BluePrints/Character/SideScrollingCharacter_Base.arrowend` _asside_scrolling_character_base)) 1000.0) false "None")
  (`KismetSystemLibrary.Delay` 3.0)
  (`GameplayStatics.SpawnEmitterAtLocation` "/Game/BluePrints/Particle/Explosion.Explosion" (`SceneComponent.K2_GetComponentLocation` (`self.Bomb`)) (struct) (5.0 5.0 5.0))
  (`self.SetActorHiddenInGame` true)
  (for _ (range 6)
    (`|SpawnActorFromClass` "/Game/BluePrints/Weapons/Bomb_Mini.Bomb_Mini_C" (`KismetMathLibrary.MakeTransform` (+ (`SceneComponent.K2_GetComponentLocation` (`self.Bomb`)) (`KismetMathLibrary.RandomUnitVector`))) "Undefined" "OverrideRootScale" null null))
  (`self.K2_DestroyActor`))

(event `self.Sphere.OnComponentHit`
  (params (HitComponent :type "PrimitiveComponent Object Reference") (OtherActor :type "Actor Object Reference") (OtherComp :type "PrimitiveComponent Object Reference") (NormalImpulse :type "Vector Structure") (Hit :type "HitResult Structure (by ref)"))
  ;[1 1 1] Bombs
  (`self.SetActorHiddenInGame` true)
  (for _ (range 6)
    (`|SpawnActorFromClass` "/Game/BluePrints/Weapons/Bomb_Mini.Bomb_Mini_C" (`KismetMathLibrary.MakeTransform` (+ (`SceneComponent.K2_GetComponentLocation` (`self.Bomb`)) (`KismetMathLibrary.RandomUnitVector`)) (struct) (1.0 1.0 1.0)) "Undefined" "OverrideRootScale" null null))
  (`self.K2_DestroyActor`))

(fn `UserConstructionScript`)
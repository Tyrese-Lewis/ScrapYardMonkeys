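; Ranged slime enemy Blueprint (DribbleGoo) that handles taking damage and dying, with no attack logic in its graphs.
; A damage macro lowers Life with a splash effect and hit montage, signalling death only when Life is already depleted as damage arrives.
; On death it plays an animation, waits briefly, then spawns a Boomerang if the player's Monkey Rage is active, otherwise increments their rage, and destroys itself.
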(event `self.ReceiveBeginPlay`
  ;[1 1 1] Reference to the player
  (bind _asside_scrolling_character_base (cast `/Game/BluePrints/Character/SideScrollingCharacter_Base` (`GameplayStatics.GetPlayerCharacter` 0)))
  (set `self.Player character Ref` _asside_scrolling_character_base))

(event `/Game/BluePrints/Interfaces/BPI_TakeDamage.TakeDamage`
  (params (Damage :type "Float (single-precision)"))
  ;[1 1 1] If damage is taken kill the enemy
  (`self.Damage To Health` Damage
    (:`True`
      (`SkeletalMeshComponent.PlayAnimation` (`self.Mesh`) "/Game/BluePrints/BP_Ai/AIEnemySlimeRanged/Anim/SlimeDeath_Montage.SlimeDeath_Montage" false)
      (`KismetSystemLibrary.Delay` 1.0)
      (if (`/Game/BluePrints/Character/SideScrollingCharacter_Base.MonkeyRageActive` (`self.Player character Ref`))
        (`|SpawnActorFromClass` "/Game/BluePrints/Weapons/Boomerang.Boomerang_C" (`SceneComponent.K2_GetComponentToWorld` (`self.CapsuleComponent`)) "Undefined" "OverrideRootScale" null null)
        (`self.K2_DestroyActor`)
        (else
          (bind _asside_scrolling_character_base (cast `/Game/BluePrints/Character/SideScrollingCharacter_Base` (`GameplayStatics.GetPlayerCharacter` 0)))
          (bind _result (`/Engine/EditorBlueprintResources/StandardMacros.IncrementFloat` (`/Game/BluePrints/Character/SideScrollingCharacter_Base.CurrentRage` _asside_scrolling_character_base))
            (:`  `
              (set `/Game/BluePrints/Character/SideScrollingCharacter_Base.CurrentRage` _result _asside_scrolling_character_base)
              (`self.K2_DestroyActor`))))))))

(fn `UserConstructionScript`)
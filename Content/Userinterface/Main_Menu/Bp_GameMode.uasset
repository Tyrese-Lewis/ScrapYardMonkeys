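; Game mode Blueprint holding draft checkpoint save and load logic for a side-scrolling character, none of which is wired to an event, so it never runs.
; The disconnected chains write either the game mode's or the player's transform to SpawnLocation in a SaveGame1_Bp slot.
; Others teleport or move the player to the saved transform, creating a save if missing, or restart the level by console command.
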(fn `UserConstructionScript`)
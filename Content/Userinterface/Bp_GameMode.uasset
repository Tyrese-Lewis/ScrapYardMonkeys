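; Game mode Blueprint that keeps an elapsed game timer, split into minutes, seconds and milliseconds.
; BeginPlay stores the current clock time as the start time, and each Tick subtracts it from the current time and breaks the difference into those three variables.
; An older manual counter that increments milliseconds and rolls them over into seconds and minutes remains in the graph but is never executed.
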(event `self.ReceiveBeginPlay`
  ;[1 1 1] Start Timer
  (set `self.StartTime` (`KismetMathLibrary.Now`)))

(event `self.ReceiveTick`
  (params (DeltaSeconds :type "Float (single-precision)"))
  ;[1 1 1] Get current time
  (bind _output_get (set `self.CurrentTime` (- (`KismetMathLibrary.Now`) (`self.StartTime`))))
  (set `self.Minutes` (`.Minutes` (`KismetMathLibrary.BreakTimespan` _output_get)))
  (set `self.Seconds` (`.Seconds` (`KismetMathLibrary.BreakTimespan` _output_get)))
  (set `self.Milliseconds` (`.Milliseconds` (`KismetMathLibrary.BreakTimespan` _output_get))))

(fn `UserConstructionScript`)